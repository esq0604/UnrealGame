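; Boss monster character that hunts the player, using a vision sphere to set or clear the AI blackboard Target and toggle its HP bar.
; ATK_01 plays a random montage; ATK_02 is a launched jump attack with temporarily widened radius.
; Both call DoDamage, a debug-drawn sphere overlap that applies damage only on the IsParry branch.
; AttackCollision applies a GAS damage effect, while taking damage activates tagged abilities and briefly swaps material.
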(event OnComponentBeginOverlap(SphereVision)
  (params (OverlappedComponent :type Primitive%20Component%20Object%20Reference) (OtherActor :type Actor%20Object%20Reference) (OtherComp :type Primitive%20Component%20Object%20Reference) (OtherBodyIndex :type Integer) (bFromSweep :type Boolean) (SweepResult :type Hit%20Result%20Structure%20%28by%20ref%29))
  ;[1 1 1] 타겟(플레이어)를 설정합니다.
  (if (!= OtherActor self)
    (if (Actor|ActorHasTag OtherActor "Player")
      (CallFunction|SetTarget OtherActor)
      (Widget|SetVisibility (Variables|Default|GetHPBarWidget) "Visible"))))

(event OnComponentEndOverlap(SphereVision)
  (params (OverlappedComponent :type Primitive%20Component%20Object%20Reference) (OtherActor :type Actor%20Object%20Reference) (OtherComp :type Primitive%20Component%20Object%20Reference) (OtherBodyIndex :type Integer))
  ;[1 1 1] 타겟(플레이어)를 지웁니다.
  (if (== OtherActor (CallFunction|GetTarget))
    (CallFunction|ClearTarget)
    (Widget|SetVisibility (Variables|Default|GetHPBarWidget) "Hidden")))

(event OnComponentBeginOverlap(AttackCollision)
  (params (OverlappedComponent :type Primitive%20Component%20Object%20Reference) (OtherActor :type Actor%20Object%20Reference) (OtherComp :type Primitive%20Component%20Object%20Reference) (OtherBodyIndex :type Integer) (bFromSweep :type Boolean) (SweepResult :type Hit%20Result%20Structure%20%28by%20ref%29))
  (if (Class|GameplayStatics|ObjectIsA OtherActor "/Script/RetargetingTest.CharacterBase")
    (GameplayEffects|ApplyGameplayEffectToTarget :self (Variables|Default|GetAbilitySystemComponent) :GameplayEffectClass "/Game/Player/GameplayEffect/GE_TwinBladeDamage.GE_TwinBladeDamage_C" :Target (Ability|GetAbilitySystemComponent OtherActor))))

(event Custom|ATK_01
  (params (Target :type Actor%20Object%20Reference))
  ;[0 0 0] ATK01
  (Utilities|FlowControl|Sequence
    (:then_0
      (Utilities|IsValid Target
        (:Is%20Valid
          (Transformation|SetActorRotation (Math|Rotator|MakeRotator 0.0 0.0 (.yaw (Math|Rotator|FindLookatRotation (Transformation|GetActorLocation) (Transformation|GetActorLocation Target))))))))
    (:then_1
      (Animation|Montage|PlayMontage (Variables|Character|GetMesh) (Utilities|Array|Get(acopy) (Variables|Attack|GetAttackArray) (Math|Random|RandomIntegerinRange 0 3))
        (:OnNotifyBegin
          (CallFunction|DoDamage))))))

(event Custom|DoDamage
  (bind _damagearrow (Variables|Default|GetDamageArrow))
  (bind _returnvalue (Transformation|GetWorldLocation _damagearrow))
  ;[1 0.03977 0.009923] Do Damage
  (bind (_outactors _returnvalue_2) (Collision|SphereOverlapActors _returnvalue (Variables|Default|GetDamageRadius) (Utilities|Array|MakeArray "ObjectTypeQuery7") 0 (Utilities|Array|MakeArray self)))
  (Rendering|Debug|DrawDebugSphere _returnvalue (Variables|Default|GetDamageRadius) 12 "(R=0.885524,G=1.000000,B=0.000000,A=1.000000)" 1.0)
  (if _returnvalue_2
    (for _array_element _outactors
      (bind _asbp_player (Utilities|Casting|CastToBP_Player _array_element))
      (if (Variables|/Game/Player/BP_Player.BP_Player_C|GetIsParry _asbp_player)
        (Animation|StopAnimMontage (Utilities|Array|Get(acopy) (Variables|Attack|GetAttackArray) (Math|Random|RandomIntegerinRange 0 3)))
        (Animation|Montage|PlayMontage (Variables|Character|GetMesh) 0
          (:then
            (Game|Damage|ApplyDamage _array_element 1.0 (Pawn|GetController) self)))
        (else
          (Development|PrintString "Player Parry False"))))))

(event Custom|ATK_02
  (params (Target :type Actor%20Object%20Reference))
  ;[1 1 1] ATK2 (Air Attack)
  (if (not (Variables|Default|GetisJumping))
    (Utilities|FlowControl|Sequence
      (:then_0
        (Utilities|IsValid Target
          (:Is%20Valid
            (Transformation|SetActorRotation (Math|Rotator|MakeRotator 0.0 0.0 (.yaw (Math|Rotator|FindLookatRotation (Transformation|GetActorLocation) (Transformation|GetActorLocation Target))))))))
      (:then_1
        (Variables|Default|SetisJumping true)
        (bind _asbp_player (Utilities|Casting|CastToBP_Player (Game|GetPlayerCharacter 0)))
        (Character|LaunchCharacter (Math|Vector|MakeVector (* (.x (Math|Vector|GetForwardVector (Variables|/Script/Engine.Actor|GetRootComponent _asbp_player))) -8e+02) (* (.y (Math|Vector|GetForwardVector (Variables|/Script/Engine.Actor|GetRootComponent _asbp_player))) -8e+02) 7e+02) true true)
        (Animation|PlayAnimMontage 0 1.0 "None")
        (Utilities|FlowControl|Delay 0.8)
        (Variables|Default|SetisJumping false)
        (Utilities|FlowControl|Delay 0.4)
        (Variables|Default|SetATK02_Active true)
        (Variables|Default|SetDamageRadius 2.5e+02)
        (Utilities|FlowControl|Delay 0.7)
        (CallFunction|DoDamage)
        (Utilities|FlowControl|Delay 0.6)
        (Variables|Default|SetDamageRadius 1e+02)
        (Variables|Default|SetATK02_Active false)))))

(event EventBeginPlay
  (bind _returnvalue (UserInterface|CreateWidget "/Game/Widgets/WBP_BossEnemyHP.WBP_BossEnemyHP_C"))
  (bind _output_get (Variables|Default|SetHPBarWidget _returnvalue))
  (UserInterface|Viewport|AddtoViewport _output_get 0)
  (Widget|SetVisibility _returnvalue "Hidden"))

(event Collision|EventActorBeginOverlap
  (params (OtherActor :type Actor%20Object%20Reference)))

(event EventTick
  (params (DeltaSeconds :type Float%20%28single-precision%29)))

(event Game|Damage|EventAnyDamage
  (params (Damage :type Float%20%28single-precision%29) (DamageType :type Damage%20Type%20Object%20Reference) (InstigatedBy :type Controller%20Object%20Reference) (DamageCauser :type Actor%20Object%20Reference))
  (Development|PrintString "takedamage")
  (Abilities|TryActivateAbilitiesbyTag (Variables|Default|GetAbilitySystemComponent) (Variables|Default|GetGameplay%20Tag%20Container) true)
  (Rendering|Material|SetMaterial (Variables|Character|GetMesh) 0 "/Game/Asset/InfinityBladeWeapons/Weapons/Blade/Swords/Blade_BlackWyrmBlade/M_Blade_BlackWyrmBlade.M_Blade_BlackWyrmBlade")
  (Utilities|FlowControl|Delay 0.5)
  (Rendering|Material|SetMaterial (Variables|Character|GetMesh) 0 0))

(fn ConstructionScript)

(fn SetTarget
  (params (NewTarget :type Actor%20Object%20Reference))
  ;[1 1 1] 블랙보드의 Target을 지정합니다.
  (AI|Components|Blackboard|SetValueasObject (AI|GetBlackboard (AI|GetAIController self)) (Utilities|Name|MakeLiteralName "Target") NewTarget))

(fn GetTarget
  ;[1 1 1] 블랙보드의 타겟을 반환합니다.
  (return (.As액터 (Utilities|Casting|CastToActor (AI|Components|Blackboard|GetValueasObject (AI|GetBlackboard (AI|GetAIController self)) (Utilities|Name|MakeLiteralName "Target"))))))

(fn ClearTarget
  ;[1 1 1] 블랙보드의 타겟을 지웁니다.
  (AI|Components|Blackboard|ClearValue (AI|GetBlackboard (AI|GetAIController self)) (Utilities|Name|MakeLiteralName "Target")))