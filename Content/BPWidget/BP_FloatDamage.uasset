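; Floating damage text actor that displays a combat text string through its Widget component.
; Its Initialize event only stores the Text, which BeginPlay passes to the WBP_CombatText widget, so the value needs to be set before BeginPlay runs.
; BeginPlay also binds to the widget's animation-finished event, with HandleAnimFinished destroying the actor once the animation completes.
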(event EventBeginPlay
  (bind _aswbp_combat_text (Utilities|Casting|CastToWBP_CombatText (UserInterface|GetUserWidgetObject (Variables|Default|GetWidget))))
  (EventDispatchers|BindEventtoAnimFinished _aswbp_combat_text (EventDispatchers|CreateEvent :!event HandleAnimFinished))
  (Default|Initialize _aswbp_combat_text (Variables|Default|GetText)))

(event Collision|EventActorBeginOverlap
  (params (OtherActor :type Actor%20Object%20Reference)))

(event EventTick
  (params (DeltaSeconds :type Float%20%28single-precision%29)))

(event EventInitialize
  (params (text :type Text%20%28by%20ref%29))
  (Variables|Default|SetText text))

(fn ConstructionScript)

(fn HandleAnimFinished
  ;[1 1 1] Destroy the actor when the animation finished
  (Actor|DestroyActor))