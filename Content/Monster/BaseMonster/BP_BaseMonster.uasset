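; Base monster Character that detects players through a vision sphere and passes them to its AI as a target.
; Overlaps by actors tagged Player write the EnemyActor blackboard key through target helper functions, and the current target leaving the sphere clears it.
; It also exposes a walk speed setter and a TestAttack montage stub with no montage assigned, and prints a debug string on every overlap.
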(event OnComponentBeginOverlap(SphereVision)
  (params (OverlappedComponent :type Primitive%20Component%20Object%20Reference) (OtherActor :type Actor%20Object%20Reference) (OtherComp :type Primitive%20Component%20Object%20Reference) (OtherBodyIndex :type Integer) (bFromSweep :type Boolean) (SweepResult :type Hit%20Result%20Structure%20%28by%20ref%29))
  (Development|PrintString "Hello")
  (if (!= OtherActor self)
    (if (Actor|ActorHasTag OtherActor "Player")
      (CallFunction|SetTarget OtherActor))))

(event OnComponentEndOverlap(SphereVision)
  (params (OverlappedComponent :type Primitive%20Component%20Object%20Reference) (OtherActor :type Actor%20Object%20Reference) (OtherComp :type Primitive%20Component%20Object%20Reference) (OtherBodyIndex :type Integer))
  (bind _target (CallFunction|GetTarget))
  (if (== _target OtherActor)
    (CallFunction|ClearTarget)))

(event EventBeginPlay)

(event Collision|EventActorBeginOverlap
  (params (OtherActor :type Actor%20Object%20Reference)))

(event EventTick
  (params (DeltaSeconds :type Float%20%28single-precision%29)))

(fn ConstructionScript)

(fn UpdateWalkSpeed
  (params (new%20walk%20speed :type Float%20%28double-precision%29))
  (Variables|/Script/Engine.CharacterMovementComponent|SetMaxWalkSpeed (Variables|Character|GetCharacterMovement) new%20walk%20speed))

(fn SetTarget
  (params (NewParam :type Actor%20Object%20Reference))
  (AI|Components|Blackboard|SetValueasObject (AI|GetBlackboard (AI|GetAIController self)) (Utilities|Name|MakeLiteralName "EnemyActor") NewParam))

(fn ClearTarget
  (AI|Components|Blackboard|ClearValue (AI|GetBlackboard (AI|GetAIController self)) (Utilities|Name|MakeLiteralName "EnemyActor")))

(fn GetTarget
  (return (.As액터 (Utilities|Casting|CastToActor (AI|Components|Blackboard|GetValueasObject (AI|GetBlackboard (AI|GetAIController self)) (Utilities|Name|MakeLiteralName "EnemyActor"))))))

(fn TestAttack
  (Animation|PlayAnimMontage 0 1.0 "None"))