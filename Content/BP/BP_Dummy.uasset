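; BP_Dummy is a dummy character that reacts to damage and can be the victim of a stealth back assassination.
; Any damage activates abilities tagged Ability.HitReaction through its Ability System; an older four-direction montage reaction is left disconnected.
; StealthBackAssasin plays an ambushed montage and returns the AssasinREF location and the dummy's rotation.
; A Ragdoll event turns on mesh physics after a delay.
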(event Custom|Ragdoll
  (Utilities|FlowControl|Delay 2.5)
  (Physics|SetSimulatePhysics (Variables|Character|GetMesh) true))

(event Collision|EventActorBeginOverlap
  (params (OtherActor :type Actor%20Object%20Reference)))

(event EventTick
  (params (DeltaSeconds :type Float%20%28single-precision%29)))

(event Game|Damage|EventAnyDamage
  (params (Damage :type Float%20%28single-precision%29) (DamageType :type Damage%20Type%20Object%20Reference) (InstigatedBy :type Controller%20Object%20Reference) (DamageCauser :type Actor%20Object%20Reference))
  (Abilities|TryActivateAbilitiesbyTag (Variables|Default|GetAbilitySystem) (GameplayTags|MakeLiteralGameplayTagContainer "(GameplayTags=((TagName=\"Ability.HitReaction\")))") true))

(event EventBeginPlay
  (bind _asplayer_state_base (Utilities|Casting|CastToPlayerStateBase (Game|GetPlayerState 0)))
  (Variables|Default|SetAs%20Player%20State%20Base _asplayer_state_base))

(fn ConstructionScript)

(fn StealthBackAssasin
  (Animation|PlayAnimMontage "/Game/Animation/Assassinations/UE5_Twinblades_Attack_Ambushed_Montage.UE5_Twinblades_Attack_Ambushed_Montage" 1.0 "None")
  (return (Transformation|GetWorldLocation (Variables|Default|GetAssasinREF)) (Transformation|GetActorRotation)))