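; GC_Damage is a gameplay cue that gives sound and particle feedback for damage.
; On execute it plays the damage sound at the cue location and spawns a body bullet-impact emitter at the hit actor's origin, taken from the effect context's hit result.
; That handler returns false without calling its parent.
; On remove it replays the sound and defers to the parent.
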(fn OnExecute
  (params (MyTarget :type Actor%20Object%20Reference) (Parameters :type Gameplay%20Cue%20Parameters%20Structure%20%28by%20ref%29))
  (bind (_normalizedmagnitude _rawmagnitude _effectcontext _matchedtagname _originaltag _aggregatedsourcetags _aggregatedtargettags _location) (Ability|GameplayCue|BreakGameplayCueParameters Parameters))
  (Audio|PlaySoundatLocation 0 (Variables|Default|GetDamageSound) _location "0, 0, 0" 1.0 1.0 0.0 0 0 0 0)
  (Effects|SpawnEmitteratLocation 0 "/Game/ShooterGame/Effects/ParticleSystems/Gameplay/Player/P_body_bullet_impact.P_body_bullet_impact" (Transformation|GetActorLocation (.hitactor (Class|AbilitySystemBlueprintLibrary|EffectContextGetHitResult _effectcontext))))
  (return false))

(fn OnRemove
  (params (MyTarget :type Actor%20Object%20Reference) (Parameters :type Gameplay%20Cue%20Parameters%20Structure%20%28by%20ref%29))
  (Audio|PlaySoundatLocation MyTarget (Variables|Default|GetDamageSound) (.Location (Ability|GameplayCue|BreakGameplayCueParameters Parameters)) "0, 0, 0" 1.0 1.0 0.0 0 0 0 0)
  (return (|CallParentFunction MyTarget Parameters)))