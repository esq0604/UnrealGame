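; Frost giant boss enemy that tracks a target and damages what its hand weapons hit.
; BeginPlay adds a boss HP bar widget with a hard-coded initial update and binds both weapon collision components to the mesh.
; OnTargeted stores the target and toggles bar visibility, while RotatetoTarget smoothly turns only yaw toward it.
; ToggleAttackCollision switches right, left or both hand collisions, whose hits apply GE_Damage through the Gameplay Ability System.
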(event OnHit(RightWeaponCollisionComp)
  (params (NewParam :type Hit%20Result%20Structure))
  (GameplayEffects|ApplyGameplayEffectToTarget :self (Variables|Default|GetAbilitySystemComponent) :GameplayEffectClass "/Game/Blueprint/GameplayEffect/GE_Damage.GE_Damage_C" :Target (Ability|GetAbilitySystemComponent (.HitActor (Collision|BreakHitResult NewParam)))))

(event OnHit(LeftWeaponCollisionComp)
  (params (NewParam :type Hit%20Result%20Structure))
  (GameplayEffects|ApplyGameplayEffectToTarget :self (Variables|Default|GetAbilitySystemComponent) :GameplayEffectClass "/Game/Blueprint/GameplayEffect/GE_Damage.GE_Damage_C" :Target (Ability|GetAbilitySystemComponent (.HitActor (Collision|BreakHitResult NewParam)))))

(event EventBeginPlay
  (bind _mesh (Variables|Character|GetMesh))
  (bind _returnvalue (UserInterface|CreateWidget "/Game/Blueprint/UI/Widgets/WBP_BossEnemyHP.WBP_BossEnemyHP_C" (Game|GetPlayerController 0)))
  (bind _output_get (Variables|Default|SetHPBarWidget _returnvalue))
  (Class|MonsterGauge|UpdateHPWidget _output_get 0.5 1.0)
  (UserInterface|Viewport|AddtoViewport _output_get 0)
  (Default|SetCollisionMeshComp (Variables|Default|GetRightWeaponCollisionComp) _mesh)
  (Default|SetCollisionMeshComp (Variables|Default|GetLeftWeaponCollisionComp) _mesh))

(event Collision|EventActorBeginOverlap
  (params (OtherActor :type Actor%20Object%20Reference)))

(event EventTick
  (params (DeltaSeconds :type Float%20%28single-precision%29)))

(event EventRotatetoTarget
  (bind _returnvalue (Transformation|GetActorRotation))
  (bind (_roll _pitch) (Math|Rotator|BreakRotator _returnvalue))
  ;[0 0 0 1 25] Rotate To Target
  (Utilities|IsValid (Variables|Default|GetTargetActor)
    (:Is%20Valid
      (Transformation|SetActorRotation (Math|Rotator|MakeRotator _roll _pitch (.yaw (Math|Interpolation|RInterpTo _returnvalue (Math|Rotator|FindLookatRotation (Transformation|GetActorLocation) (Transformation|GetActorLocation (Variables|Default|GetTargetActor))) (Utilities|Time|GetWorldDeltaSeconds) 9.0)))))))

(event EventOnTargeted
  (params (NewTarget :type Actor%20Object%20Reference))
  ;[0 0 0 1 28] TargetSet && SetHealthBarVisible
  (Variables|Default|SetTargetActor NewTarget)
  (Widget|SetVisibility (Variables|Default|GetHPBarWidget) (select (Utilities|IsValid NewTarget) "Visible" "Collapsed")))

(event EventToggleAttackCollision
  (params (bCollisionEnable :type Boolean) (CollisionPart :type E_CollisionPart%20Enum :default "NewEnumerator0"))
  (switch Utilities|FlowControl|Switch|SwitchonE_CollisionPart CollisionPart
    (:NewEnumerator0
      (Default|SetCollisionEnable (Variables|Default|GetRightWeaponCollisionComp) bCollisionEnable))
    (:NewEnumerator1
      (Default|SetCollisionEnable (Variables|Default|GetLeftWeaponCollisionComp) bCollisionEnable))
    (:NewEnumerator2
      (Default|SetCollisionEnable (Variables|Default|GetRightWeaponCollisionComp) bCollisionEnable)
      (Default|SetCollisionEnable (Variables|Default|GetLeftWeaponCollisionComp) bCollisionEnable))))

(fn ConstructionScript)