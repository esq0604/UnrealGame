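; AI controller for boss enemies that starts the possessed monster's behavior tree.
; On possession it casts the pawn to BaseMonster, caches it and runs the BehaviorTree asset that the monster supplies.
; The AI perception update event is empty; leftover nodes for writing the Blackboard "Target" key and the monster's TargetActor are disconnected and never run.
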(event OnTargetPerceptionUpdated(AIPerceptionComponent)
  (params (Actor :type Actor%20Object%20Reference) (Stimulus :type AI%20Stimulus%20Structure)))

(event EventBeginPlay)

(event EventTick
  (params (DeltaSeconds :type Float%20%28single-precision%29)))

(event EventPossess
  (params (PossessedPawn :type Pawn%20Object%20Reference))
  (bind _asbase_monster (Utilities|Casting|CastToBaseMonster PossessedPawn))
  (Variables|Default|SetAs%20Base%20Monster _asbase_monster)
  (AI|RunBehaviorTree (Variables|/Script/RetargetingTest.BaseMonster|GetBehaviorTree _asbase_monster)))

(fn ConstructionScript)