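; Base enemy character Blueprint with targetable marker, AI target storage, melee attacks, hit reactions and death.
; Toggleable left and right weapon collisions apply a GAS damage effect plus point damage to hit actors.
; Incoming point damage shows floating text through the attacker's component, then plays front or back montages by dot product.
; At zero attribute value, it updates the AI blackboard, disables movement and activates death abilities by tag.
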(event OnHit(RightWeaponColliison)
  (params (NewParam :type Hit%20Result%20Structure))
  (CallFunction|ApplyDamageEffect NewParam))

(event OnHit(LeftWeaponCollision)
  (params (NewParam :type Hit%20Result%20Structure))
  (CallFunction|ApplyDamageEffect NewParam))

(event Custom|PerformHitReaction
  (params (HitFront? :type Boolean))
  ;[0 0 0 1 20] HitReaction
  (if HitFront?
    (bind _hitreactionfront (Variables|Default|GetHitReactionFront)
      (:then
        (Animation|PlayAnimMontage _hitreactionfront 1.0 "None"))
      (:else))
    (else
      (bind _hitreactionback (Variables|Default|GetHitReactionBack)
        (:then
          (Animation|PlayAnimMontage _hitreactionback 1.0 "None"))
        (:else)))))

(event EventBeginPlay
  (Rendering|SetVisibility (Variables|Default|GetTargetWidget) false false)
  (Rendering|SetVisibility (Variables|Default|GetHPWidgetComponent) false false))

(event Collision|EventActorBeginOverlap
  (params (OtherActor :type Actor%20Object%20Reference)))

(event EventTick
  (params (DeltaSeconds :type Float%20%28single-precision%29)))

(event EventOnTargeted
  (params (IsTargeted :type Boolean))
  ;[1 1 1] 플레이어의 타게팅 컴포넌트로 지정될시 호출됩니다.
  (Rendering|SetVisibility (Variables|Default|GetTargetWidget) IsTargeted false))

(event EventToggleAttackCollision
  (params (bCollisionEnable :type Boolean) (CollisionPart :type E_CollisionPart%20Enum :default "NewEnumerator0"))
  (switch Utilities|FlowControl|Switch|SwitchonE_CollisionPart CollisionPart
    (:NewEnumerator0
      (Default|SetCollisionEnable (Variables|Default|GetRightWeaponColliison) bCollisionEnable))
    (:NewEnumerator1
      (Default|SetCollisionEnable (Variables|Default|GetLeftWeaponCollision) bCollisionEnable))
    (:NewEnumerator2
      (Default|SetCollisionEnable (Variables|Default|GetRightWeaponColliison) bCollisionEnable)
      (Default|SetCollisionEnable (Variables|Default|GetLeftWeaponCollision) bCollisionEnable))))

(event Game|Damage|EventPointDamage
  (params (Damage :type Float%20%28single-precision%29) (DamageType :type Damage%20Type%20Object%20Reference) (HitLocation :type Vector :default "0, 0, 0") (HitNormal :type Vector :default "0, 0, 0") (HitComponent :type Primitive%20Component%20Object%20Reference) (BoneName :type Name :default "None") (ShotFromDirection :type Vector :default "0, 0, 0") (InstigatedBy :type Controller%20Object%20Reference) (DamageCauser :type Actor%20Object%20Reference) (HitInfo :type Hit%20Result%20Structure%20%28by%20ref%29))
  (CallFunction|HandleDamage (Pawn|GetControlledPawn InstigatedBy) Damage)
  ;[0 0 0 1 20] HitReaction
  (if (<= (.ReturnValue (Ability|Attribute|GetFloatAttributefromAbilitySystemComponent (Variables|Default|GetAbilitySystemComponent) "(AttributeName=\"Health\",Attribute=/Script/RetargetingTest.BaseAttributeSet:Health,AttributeOwner=/Script/CoreUObject.Class'\"/Script/RetargetingTest.BaseAttributeSet\"')")) 0.0)
    (CallFunction|SetDeath true)
    (else
      (bind _output_get (Variables|Default|SetHitFront? (Math|Float|InRange(Float) (Class|Actor|GetDotProductto self (Pawn|GetControlledPawn InstigatedBy)) 0.0 1.0)))
      (CallFunction|PerformHitReaction _output_get))))

(fn ConstructionScript)

(fn OnTargetSet
  (params (NewTargetActor :type Actor%20Object%20Reference))
  ;[1 1 1] AI퍼셉션으로 발견시 호출됩니다.
  (Variables|Default|SetTargetActor NewTargetActor))

(fn ApplyDamageEffect
  (params (Hit :type Hit%20Result%20Structure%20%28by%20ref%29))
  (bind _hitactor (Collision|BreakHitResult Hit))
  (bind _returnvalue (Class|BPICombat|CanReciveDamage(Message) _hitactor))
  (if _returnvalue
    (GameplayEffects|ApplyGameplayEffectToTarget :self (Variables|Default|GetAbilitySystemComponent) :GameplayEffectClass "/Game/Blueprint/GameplayEffect/GE_Damage.GE_Damage_C" :Target (Ability|GetAbilitySystemComponent _hitactor))
    (Game|Damage|ApplyPointDamage _hitactor 1.0 (Transformation|GetActorForwardVector) Hit (Game|GetInstigatorController) self)))

(fn SetDeath
  (params (IsDead :type Boolean))
  (if IsDead
    (bind _output_get (Variables|Default|SetIsDead (!= IsDead (Variables|Default|GetIsDead))))
    (AI|Components|Blackboard|SetValueasBool (AI|GetBlackboard (AI|GetAIController self)) (LocalVariables|GetbIsDead) _output_get)
    (Pawn|Components|CharacterMovement|SetMovementMode (Variables|Character|GetCharacterMovement) "MOVE_None" 0)
    (Abilities|TryActivateAbilitiesbyTag (Variables|Default|GetAbilitySystemComponent) (Variables|Default|GetDeadTag) true)))

(fn HandleDamage
  (params (DamageCauser :type Actor%20Object%20Reference) (Damage :type Float%20%28double-precision%29))
  (Utilities|FlowControl|Sequence
    (:then_0
      (LocalVariables|SetDamageCauserFloatinComp (Actor|GetComponentbyClass DamageCauser "/Script/RetargetingTest.FloatingCombatTextComponent")))
    (:then_1
      (bind _damagecauserfloatincomp (LocalVariables|GetDamageCauserFloatinComp)
        (:then
          (Class|FloatingCombatTextComponent|AddFloatingActor _damagecauserfloatincomp (Utilities|Text|ToText(Float) Damage "HalfToEven") (Transformation|GetActorLocation)))
        (:else)))))

(fn CanbeTargeted?
  (return (not (Variables|Default|GetIsDead))))

(fn CanReciveDamage
  (return false))

(fn GetHitReaction
  (params (HitDirection :type Enum_HitDirection%20Enum :default "NewEnumerator0"))
  (return 0))

(fn GetUseItemTag
  (return ""))

(fn UseItembyTag
  (params (ItemTag :type Gameplay%20Tag%20Structure))
  (return false))