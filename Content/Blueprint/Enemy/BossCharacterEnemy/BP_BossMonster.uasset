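; Boss monster enemy Blueprint with helper functions that set, get and clear the Target key in its AI controller's Blackboard.
; Its event graph holds logic to apply a GAS damage effect to hit characters, and to track Player-tagged actors as targets while toggling the HP bar widget.
; None of that event graph logic runs, so only the Blackboard helpers are usable as written.
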(fn ConstructionScript)

(fn SetTarget
  (params (NewTarget :type Actor%20Object%20Reference))
  (AI|Components|Blackboard|SetValueasObject (AI|GetBlackboard (AI|GetAIController self)) (Utilities|Name|MakeLiteralName "Target") NewTarget))

(fn GetTarget
  ;[1 1 1] 블랙보드의 타겟을 반환합니다.
  (return (.As액터 (Utilities|Casting|CastToActor (AI|Components|Blackboard|GetValueasObject (AI|GetBlackboard (AI|GetAIController self)) (Utilities|Name|MakeLiteralName "Target"))))))

(fn ClearTarget
  ;[1 1 1] 블랙보드의 타겟을 지웁니다.
  (AI|Components|Blackboard|ClearValue (AI|GetBlackboard (AI|GetAIController self)) (Utilities|Name|MakeLiteralName "Target")))