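; BP_BossAIController is the AI controller for a boss enemy, feeding perceived targets into its Blackboard.
; On perception updates, successfully sensed Damage or Sight stimuli write the sensed actor to the TargetActor key, with debug prints.
; Lost stimuli leave the key unchanged.
; Possess only calls the parent; the nodes that run the BaseMonster's behavior tree asset are disconnected.
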(event OnTargetPerceptionUpdated(AIPerception)
  (params (Actor :type Actor%20Object%20Reference) (Stimulus :type AI%20Stimulus%20Structure))
  (Development|PrintString "perception update")
  (if (.bSuccessfullySensed (Utilities|Struct|BreakAIStimulus Stimulus))
    (bind _returnvalue (Class|AIPerceptionSystem|GetSenseClassforStimulus Stimulus))
    (if (== _returnvalue "/Script/AIModule.AISense_Damage")
      (AI|Components|Blackboard|SetValueasObject (Variables|Default|GetBlackboard) (Utilities|Name|MakeLiteralName "TargetActor") Actor :!label _label)
      (Development|PrintString "set target")
      (else
        (bind _returnvalue_2 (Class|AIPerceptionSystem|GetSenseClassforStimulus Stimulus))
        (if (== _returnvalue_2 "/Script/AIModule.AISense_Sight")
          (goto _label))))))

(event EventTick
  (params (DeltaSeconds :type Float%20%28single-precision%29)))

(event EventPossess
  (params (PossessedPawn :type Pawn%20Object%20Reference))
  (|CallParentFunction PossessedPawn))

(fn ConstructionScript)