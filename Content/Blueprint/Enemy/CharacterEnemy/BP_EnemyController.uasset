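; Enemy AI controller that runs the BT_Enemy behavior tree when it possesses a pawn.
; Unconnected perception logic would store a sensed Player-tagged actor in blackboard keys EnemyActor and HasLineOfSight, otherwise start a line-of-sight grace timer.
; That timer's event clears both keys to end the chase.
; The perception update event is empty, so this detection and timer logic never runs.
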(event OnTargetPerceptionUpdated(AIPerception)
  (params (Actor :type Actor%20Object%20Reference) (Stimulus :type AI%20Stimulus%20Structure)))

(event Custom|StartEnemyTimer
  (bind _blackboard (Variables|Default|GetBlackboard))
  ;[1 1 1] 플레이어가 시야에 없어져도 Line Of Sight Timer동안 추격을 포기하지 않습니다.
  (AI|Components|Blackboard|SetValueasBool _blackboard (Variables|Default|GetHasLineOfSight) false)
  (AI|Components|Blackboard|SetValueasObject _blackboard (Variables|Default|GetEnemyActor) 0))

(event EventBeginPlay)

(event EventTick
  (params (DeltaSeconds :type Float%20%28single-precision%29)))

(event EventPossess
  (params (PossessedPawn :type Pawn%20Object%20Reference))
  (AI|RunBehaviorTree "/Game/Blueprint/Enemy/CharacterEnemy/BT_Enemy.BT_Enemy"))

(fn ConstructionScript)