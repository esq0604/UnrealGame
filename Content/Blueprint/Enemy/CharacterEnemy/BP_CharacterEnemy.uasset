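; Enemy character Blueprint that extends a parent combat character with a melee weapon, HP widget and Twinblades hit reactions.
; BeginPlay binds the weapon mesh to the right weapon collision component.
; Being targeted or acquiring a target through AI perception shows the HP widget, with no hide logic here.
; RotatetoTarget smoothly yaws toward a targetable actor, and GetHitReaction maps hit direction to left or right montages.
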(event EventOnTargeted
  (params (IsTargeted :type Boolean))
  ;[1 1 1] 타게팅컴포넌트로 지정될때 호출됩니다.
  (|CallParentFunction IsTargeted)
  (Rendering|SetVisibility (Variables|Default|GetHPWidgetComponent) true false))

(event EventToggleAttackCollision
  (params (bCollisionEnable :type Boolean) (CollisionPart :type E_CollisionPart%20Enum :default "NewEnumerator0"))
  (|CallParentFunction bCollisionEnable CollisionPart))

(event EventBeginPlay
  (|CallParentFunction)
  (Default|SetCollisionMeshComp (Variables|Default|GetRightWeaponColliison) (Variables|Default|GetWeaponMesh)))

(event EventRotatetoTarget
  (bind _returnvalue (Transformation|GetActorRotation))
  (bind _targetactor (Variables|Default|GetTargetActor))
  (bind (_roll _pitch) (Math|Rotator|BreakRotator _returnvalue))
  (Utilities|IsValid _targetactor
    (:Is%20Valid
      (bind _returnvalue_2 (Class|BPITargeting|CanbeTargeted?(Message) _targetactor))
      (if _returnvalue_2
        (Transformation|SetActorRotation (Math|Rotator|MakeRotator _roll _pitch (.yaw (Math|Interpolation|RInterpTo _returnvalue (Math|Rotator|FindLookatRotation (Transformation|GetActorLocation) (Transformation|GetActorLocation (Variables|Default|GetTargetActor))) (Utilities|Time|GetWorldDeltaSeconds) 9.0))))))))

(fn ConstructionScript)

(fn UpdateWalkSpeed
  (params (new%20walk%20speed :type Float%20%28double-precision%29))
  (Variables|/Script/Engine.CharacterMovementComponent|SetMaxWalkSpeed (Variables|Character|GetCharacterMovement) new%20walk%20speed))

(fn OnTargetSet
  (params (NewTargetActor :type Actor%20Object%20Reference))
  ;[1 1 1] AI퍼셉션으로 발견시 호출됩니다.
  (|CallParentFunction NewTargetActor)
  (Rendering|SetVisibility (Variables|Default|GetHPWidgetComponent) true false))

(fn GetHitReaction
  (params (HitDirection :type Enum_HitDirection%20Enum :default "NewEnumerator0"))
  (switch Utilities|FlowControl|Switch|SwitchonEnum_HitDirection HitDirection
    (:NewEnumerator0
      (return "/Game/Asset/Animation/TwinbladesAnimsetBase/InPlace/Twinblades_Hit_Right_Montage.Twinblades_Hit_Right_Montage"))
    (:NewEnumerator1
      (return "/Game/Asset/Animation/TwinbladesAnimsetBase/InPlace/Twinblades_Hit_Right_Montage.Twinblades_Hit_Right_Montage"))
    (:NewEnumerator2
      (return "/Game/Asset/Animation/TwinbladesAnimsetBase/InPlace/Twinblades_Hit_Left_Montage.Twinblades_Hit_Left_Montage"))
    (:NewEnumerator3
      (return "/Game/Asset/Animation/TwinbladesAnimsetBase/InPlace/Twinblades_Hit_Right_Montage.Twinblades_Hit_Right_Montage"))))