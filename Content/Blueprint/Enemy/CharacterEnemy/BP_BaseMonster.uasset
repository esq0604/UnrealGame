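; BP_BaseMonster is a base enemy character driven by an AI blackboard and the Gameplay Ability System.
; SphereVision overlap with a Player-tagged actor writes it to the EnemyActor blackboard key through target helper functions.
; AnyDamage and TestAttack activate abilities by tag, and UpdateWalkSpeed sets movement speed.
; Target clearing on overlap end and the death montage, hide and destroy steps are disconnected, so they never run.
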(event OnComponentBeginOverlap(SphereVision)
  (params (OverlappedComponent :type Primitive%20Component%20Object%20Reference) (OtherActor :type Actor%20Object%20Reference) (OtherComp :type Primitive%20Component%20Object%20Reference) (OtherBodyIndex :type Integer) (bFromSweep :type Boolean) (SweepResult :type Hit%20Result%20Structure%20%28by%20ref%29))
  ;[1 1 1] 코멘트
  (if (!= OtherActor self)
    (if (Actor|ActorHasTag OtherActor "Player")
      (CallFunction|SetTarget OtherActor))))

(event OnComponentEndOverlap(SphereVision)
  (params (OverlappedComponent :type Primitive%20Component%20Object%20Reference) (OtherActor :type Actor%20Object%20Reference) (OtherComp :type Primitive%20Component%20Object%20Reference) (OtherBodyIndex :type Integer))
  ;[1 1 1] 코멘트
)

(event EventBeginPlay
  (Transformation|AttachComponentToComponent (Variables|Default|GetAttackCollision) (Variables|Default|GetCapsuleComponent) "None" "KeepRelative" "KeepRelative" "KeepRelative" true))

(event Game|Damage|EventAnyDamage
  (params (Damage :type Float%20%28single-precision%29) (DamageType :type Damage%20Type%20Object%20Reference) (InstigatedBy :type Controller%20Object%20Reference) (DamageCauser :type Actor%20Object%20Reference))
  (bind _abilitysystemcomponent (Variables|Default|GetAbilitySystemComponent))
  ;[1 1 1] 코멘트
  ;;[1 1 1] 해당 이벤트는 액터클래스의 리시브데미지라는 함수이고 C++에서 사용하는 테이크데미지는 따로있는것
  (Abilities|TryActivateAbilitiesbyTag _abilitysystemcomponent (Variables|Default|GetGameplay%20Tag%20Container) true)
  (if (<= (.ReturnValue (Ability|Attribute|GetFloatAttributefromAbilitySystemComponent _abilitysystemcomponent "(AttributeName=\"Health\",Attribute=/Script/RetargetingTest.EnemyAttributeSetBase:Health,AttributeOwner=/Script/CoreUObject.Class'\"/Script/RetargetingTest.EnemyAttributeSetBase\"')")) 0.0)
    _))

(fn ConstructionScript)

(fn UpdateWalkSpeed
  (params (new%20walk%20speed :type Float%20%28double-precision%29))
  (Variables|/Script/Engine.CharacterMovementComponent|SetMaxWalkSpeed (Variables|Character|GetCharacterMovement) new%20walk%20speed))

(fn SetTarget
  (params (NewParam :type Actor%20Object%20Reference))
  (AI|Components|Blackboard|SetValueasObject (AI|GetBlackboard (AI|GetAIController self)) (Utilities|Name|MakeLiteralName "EnemyActor") NewParam))

(fn ClearTarget
  (AI|Components|Blackboard|ClearValue (AI|GetBlackboard (AI|GetAIController self)) (Utilities|Name|MakeLiteralName "EnemyActor")))

(fn GetTarget
  (return (.As액터 (Utilities|Casting|CastToActor (AI|Components|Blackboard|GetValueasObject (AI|GetBlackboard (AI|GetAIController self)) (Utilities|Name|MakeLiteralName "EnemyActor"))))))

(fn TestAttack
  (Abilities|TryActivateAbilitiesbyTag (Variables|Default|GetAbilitySystemComponent) (Variables|Default|GetAttack%20Tag%20Container) true))