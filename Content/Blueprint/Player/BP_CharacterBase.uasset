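; BP_CharacterBase is a base player character Blueprint that exposes Gameplay Ability System attributes for health, mana and stamina.
; On BeginPlay it casts its PlayerState to PlayerStateBase and caches that state's Ability System Component.
; Getter functions read float attributes from the cached component and also return each as a ratio against a second attribute read.
; Blocking and FinishedBlocking are empty stubs.
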(event EventBeginPlay
  (bind _asplayer_state_base (Utilities|Casting|CastToPlayerStateBase (Variables|Default|GetPlayerState)))
  (bind _output_get (Variables|Default|SetAs%20Player%20State%20Base _asplayer_state_base))
  (Variables|Default|SetAbilitySystemComp (Ability|GetAbilitySystemComponent _output_get)))

(event Collision|EventActorBeginOverlap
  (params (OtherActor :type Actor%20Object%20Reference)))

(event EventTick
  (params (DeltaSeconds :type Float%20%28single-precision%29)))

(fn ConstructionScript)

(fn Blocking)

(fn FinishedBlocking)

(fn GetHealth
  (return (.ReturnValue (Ability|Attribute|GetFloatAttributefromAbilitySystemComponent (Variables|Default|GetAbilitySystemComp) "(AttributeName=\"Health\",Attribute=/Script/RetargetingTest.RuneAttributeSet:Health,AttributeOwner=/Script/CoreUObject.Class'\"/Script/RetargetingTest.RuneAttributeSet\"')"))))

(fn GetHealthasRatio
  (bind _result (CallFunction|GetHealth))
  (return (/ _result (.ReturnValue (Ability|Attribute|GetFloatAttributefromAbilitySystemComponent (Variables|Default|GetAbilitySystemComp) "(AttributeName=\"MaxHealth\",Attribute=/Script/RetargetingTest.RuneAttributeSet:MaxHealth,AttributeOwner=/Script/CoreUObject.Class'\"/Script/RetargetingTest.RuneAttributeSet\"')")))))

(fn GetMana
  (return (.ReturnValue (Ability|Attribute|GetFloatAttributefromAbilitySystemComponent (Variables|Default|GetAbilitySystemComp) "(AttributeName=\"Mana\",Attribute=/Script/RetargetingTest.RuneAttributeSet:Mana,AttributeOwner=/Script/CoreUObject.Class'\"/Script/RetargetingTest.RuneAttributeSet\"')"))))

(fn GetManaasRatio
  (bind _result (CallFunction|GetMana))
  (return (/ _result (.ReturnValue (Ability|Attribute|GetFloatAttributefromAbilitySystemComponent (Variables|Default|GetAbilitySystemComp) "(AttributeName=\"MaxMana\",Attribute=/Script/RetargetingTest.CharacterAttributeSetBase:MaxMana,AttributeOwner=/Script/CoreUObject.Class'\"/Script/RetargetingTest.CharacterAttributeSetBase\"')")))))

(fn GetStamina
  (return (.ReturnValue (Ability|Attribute|GetFloatAttributefromAbilitySystemComponent (Variables|Default|GetAbilitySystemComp) "(AttributeName=\"Stamina\",Attribute=/Script/RetargetingTest.RuneAttributeSet:Stamina,AttributeOwner=/Script/CoreUObject.Class'\"/Script/RetargetingTest.RuneAttributeSet\"')"))))

(fn GetStaminaasRatio
  (bind _result (CallFunction|GetStamina))
  (return (/ _result (.ReturnValue (Ability|Attribute|GetFloatAttributefromAbilitySystemComponent (Variables|Default|GetAbilitySystemComp) "(AttributeName=\"MaxStamina\",Attribute=/Script/RetargetingTest.RuneAttributeSet:MaxStamina,AttributeOwner=/Script/CoreUObject.Class'\"/Script/RetargetingTest.RuneAttributeSet\"')")))))