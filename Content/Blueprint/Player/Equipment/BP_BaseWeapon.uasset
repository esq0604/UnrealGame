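; BP_BaseWeapon is a base equippable melee-style weapon that deals damage through the Gameplay Ability System.
; On equip it hands its item static mesh to a collision component, which ToggleWeaponCollision switches on and off.
; Each valid hit from that component applies GE_Damage from the owner's ability system to the hit actor's.
; It also reports an AI damage sense event with the owner as instigator and event location.
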(event OnHit(BP_CollisionComponent)
  (params (NewParam :type Hit%20Result%20Structure))
  (bind _hitactor (Collision|BreakHitResult NewParam))
  (bind _returnvalue (Components|GetOwner))
  (if (Utilities|IsValid _hitactor)
    (GameplayEffects|ApplyGameplayEffectToTarget :self (Ability|GetAbilitySystemComponent (Components|GetOwner)) :GameplayEffectClass "/Game/Blueprint/GameplayEffect/GE_Damage.GE_Damage_C" :Target (Ability|GetAbilitySystemComponent _hitactor))
    (Class|AISenseDamage|ReportDamageEvent _hitactor _returnvalue 0.0 (Transformation|GetActorLocation _returnvalue) "0, 0, 0" "None")))

(event Custom|ToggleWeaponCollision
  (params (Condition :type Boolean))
  (Default|SetCollisionEnable (Variables|Default|GetBP_CollisionComponent) Condition))

(event EventBeginPlay
  (|CallParentFunction) ; 지금 이 노드는 비활성 상태입니다. \n핀을 끌어서 다른 노드를 연결하면 활성화됩니다.
)

(event Collision|EventActorBeginOverlap
  (params (OtherActor :type Actor%20Object%20Reference))
  (|CallParentFunction OtherActor) ; 지금 이 노드는 비활성 상태입니다. \n핀을 끌어서 다른 노드를 연결하면 활성화됩니다.
)

(event EventTick
  (params (DeltaSeconds :type Float%20%28single-precision%29))
  (|CallParentFunction DeltaSeconds) ; 지금 이 노드는 비활성 상태입니다. \n핀을 끌어서 다른 노드를 연결하면 활성화됩니다.
)

(fn ConstructionScript
  (|CallParentFunction))

(fn OnEquipped
  (|CallParentFunction)
  (Default|SetCollisionMeshComp (Variables|Default|GetBP_CollisionComponent) (Variables|Default|GetItemStaticMeshComp)))