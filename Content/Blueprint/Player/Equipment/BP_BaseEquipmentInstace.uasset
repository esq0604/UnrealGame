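; Base equipment instance Blueprint for player gear that attaches to the owning character.
; OnEquipped casts the owner to Character and snaps the equipment to the configured socket on its mesh.
; Getters expose the equipped flag, which nothing here sets, and the owned gameplay tags, with a non-exact tag match check.
; UnEquipped and PerformItemAction are empty stubs.
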(event Custom|PerformItemAction)

(event EventBeginPlay)

(event Collision|EventActorBeginOverlap
  (params (OtherActor :type Actor%20Object%20Reference)))

(event EventTick
  (params (DeltaSeconds :type Float%20%28single-precision%29)))

(fn ConstructionScript)

(fn OnEquipped
  (bind _as캐릭터 (Utilities|Casting|CastToCharacter (Components|GetOwner)))
  (Transformation|AttachComponentToComponent (Variables|/Script/Engine.Character|GetMesh _as캐릭터) (Variables|Initialization|GetAttachSocketName) "SnapToTarget" "SnapToTarget" "SnapToTarget" true))

(fn UnEquipped)

(fn GetIsEquipped
  (return (Variables|Default|GetbIsEquipped)))

(fn GetOwnedGameplayTag
  (return (Variables|Default|GetOwnedGameplayTag)))

(fn HasMachingGameplayTag
  (params (TagToCheck :type Gameplay%20Tag%20Structure))
  (return (GameplayTags|HasTag (Variables|Default|GetOwnedGameplayTag) TagToCheck)))