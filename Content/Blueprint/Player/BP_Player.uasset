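; Player character Blueprint for melee combat with a spawned twin-blade weapon, vaulting and Gameplay Ability System effects.
; Vault probes the obstacle with forward and downward traces, then feeds start, middle and landing points to Motion Warping during a collision-free montage.
; Point damage triggers front or back hit-reaction abilities, or ragdoll death at a zero attribute; an IFrame flag gates damage.
; Parry, assassination and older block-reaction logic remain disconnected.
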(event Custom|VaultMotionWarp
  (bind _mesh (Variables|Character|GetMesh))
  (bind _returnvalue (Transformation|GetWorldLocation _mesh))
  ;[1 1 1] 코멘트
  (if (and (Variables|Vault|GetCan%20Warp) (Math|Float|InRange(Float) (.z (Variables|Vault|GetVault%20Land%20Pos)) (- (.z _returnvalue) 5e+01) (+ (.z _returnvalue) 5e+01)))
    (Pawn|Components|CharacterMovement|SetMovementMode (Variables|Character|GetCharacterMovement) "MOVE_Flying" 0)
    (Collision|SetActorEnableCollision false)
    (Class|MotionWarpingComponent|AddorUpdateWarpTarget (Variables|Default|GetMotionWarpComponent) (Utilities|Struct|MakeMotionWarpingTarget "VaultStart" (Variables|Vault|GetVault%20Start%20Pos) (Transformation|GetActorRotation) 0 "None" false))
    (Class|MotionWarpingComponent|AddorUpdateWarpTarget (Variables|Default|GetMotionWarpComponent) (Utilities|Struct|MakeMotionWarpingTarget "VaultMiddle" (Variables|Vault|GetVault%20Middle%20Pos) (Transformation|GetActorRotation) 0 "None" false))
    (Class|MotionWarpingComponent|AddorUpdateWarpTarget (Variables|Default|GetMotionWarpComponent) (Utilities|Struct|MakeMotionWarpingTarget "VaultLand" (Variables|Vault|GetVault%20Land%20Pos) (Transformation|GetActorRotation) 0 "None" false))
    (Animation|Montage|PlayMontage (Variables|Character|GetMesh) 0
      (:OnCompleted
        (Pawn|Components|CharacterMovement|SetMovementMode (Variables|Character|GetCharacterMovement) "MOVE_Walking" 0)
        (Collision|SetActorEnableCollision true)
        (Variables|Vault|SetCan%20Warp false)
        ;;[1 1 1] 랜딩포지션이 애니메이션 실행후 업데이트되지 않음으로,
        (Variables|Vault|SetVault%20Land%20Pos "0.000000,0.000000,20000.000000")))))

(event Custom|PerformDead
  (bind _asabp_character (Utilities|Casting|CastToABP_Character (Components|SkeletalMesh|GetAnimInstance (Variables|Character|GetMesh))))
  (Default|SetDead _asabp_character true)
  (Input|DisableInput (Pawn|GetController) 0)
  (Pawn|Components|CharacterMovement|DisableMovement (Variables|Character|GetCharacterMovement))
  (Collision|SetCollisionResponsetoChannel (Variables|Default|GetCapsuleComponent) "ECC_GameTraceChannel2" "ECR_Ignore")
  (Collision|SetCollisionProfileName (Variables|Character|GetMesh) "ragdoll" true :!class /Script/Engine.PrimitiveComponent))

(event Input|EnhancedActionEvents|EnhancedInputActionIA_Vaut
  (params (ActionValue :type Boolean) (ElapsedSeconds :type Float%20%28double-precision%29) (TriggeredSeconds :type Float%20%28double-precision%29) (InputAction :type Input%20Action%20Object%20Reference :default "/Game/Input/Actions/IA_Vaut.IA_Vaut"))
  ;[1 1 1] Vault
  (:Started
    (CallFunction|Vault)))

(event Input|EnhancedActionEvents|EnhancedInputActionIA_Assassination
  (params (ActionValue :type Boolean) (ElapsedSeconds :type Float%20%28double-precision%29) (TriggeredSeconds :type Float%20%28double-precision%29) (InputAction :type Input%20Action%20Object%20Reference :default "/Game/Input/Actions/IA_Assassination.IA_Assassination"))
  ;[1 1 1] Stealth Assasination
)

(event Game|Damage|EventAnyDamage
  (params (Damage :type Float%20%28single-precision%29) (DamageType :type Damage%20Type%20Object%20Reference) (InstigatedBy :type Controller%20Object%20Reference) (DamageCauser :type Actor%20Object%20Reference))
  ;[1 1 1] 코멘트
)

(event EventBeginPlay
  (bind _self self)
  (bind _returnvalue (Game|SpawnActorfromClass "/Game/Blueprint/Player/Equipment/BP_TwinBladeWeapon.BP_TwinBladeWeapon_C" (Transformation|GetActorTransform) "Undefined" _self _self))
  (bind _output_get (Variables|Default|SetMainWeapon _returnvalue))
  (Default|OnEquipped _output_get))

(event EventOnLanded
  (params (Hit :type Hit%20Result%20Structure%20%28by%20ref%29))
  ;[1 1 1] 게임시작시 LinkAnimLayer를 설정해주어 BaseLayer의 플레이할 시퀀스를 동적으로 할당해줍니다.
  (GameplayEffects|ApplyGameplayEffectToSelf :self (Variables|Default|GetAbilitySystemComponent) :GameplayEffectClass "/Game/Blueprint/GameplayEffect/GE_IsGround.GE_IsGround_C"))

(event EventSetIFrame
  (params (NewIFrame :type Boolean))
  (Variables|Default|SetIFrame NewIFrame))

(event EventToggleAttackCollision
  (params (bCollisionEnable :type Boolean) (CollisionPart :type E_CollisionPart%20Enum :default "NewEnumerator0"))
  (switch Utilities|FlowControl|Switch|SwitchonE_CollisionPart CollisionPart
    (:NewEnumerator0
      (Default|SetCollisionEnable (Variables|/Game/Blueprint/Player/Equipment/BP_BaseWeapon.BP_BaseWeapon_C|GetBP_CollisionComponent (Variables|Default|GetMainWeapon)) bCollisionEnable))))

(event Game|Damage|EventPointDamage
  (params (Damage :type Float%20%28single-precision%29) (DamageType :type Damage%20Type%20Object%20Reference) (HitLocation :type Vector :default "0, 0, 0") (HitNormal :type Vector :default "0, 0, 0") (HitComponent :type Primitive%20Component%20Object%20Reference) (BoneName :type Name :default "None") (ShotFromDirection :type Vector :default "0, 0, 0") (InstigatedBy :type Controller%20Object%20Reference) (DamageCauser :type Actor%20Object%20Reference) (HitInfo :type Hit%20Result%20Structure%20%28by%20ref%29))
  ;[0 0 0 1 20] HitReaction
  (GameplayEffects|RemoveActiveEffectswithGrantedTags (Variables|Default|GetAbilitySystemComponent) "(GameplayTags=((TagName=\"Ability.State.Combo1\"),(TagName=\"Ability.State.Combo2\"),(TagName=\"Ability.State.Combo3\"),(TagName=\"Ability.State.Combo4\")))")
  (if (<= (.ReturnValue (Ability|Attribute|GetFloatAttributefromAbilitySystemComponent 0 "(AttributeName=\"Health\",Attribute=/Script/RetargetingTest.BaseAttributeSet:Health,AttributeOwner=/Script/CoreUObject.Class'\"/Script/RetargetingTest.BaseAttributeSet\"')")) 0.0)
    (CallFunction|PerformDead)
    (else
      (bind _output_get (Variables|Default|SetHitFront? (Math|Float|InRange(Float) (Class|Actor|GetDotProductto self (Pawn|GetControlledPawn InstigatedBy)) 0.0 1.0)))
      (if _output_get
        (Abilities|TryActivateAbilitiesbyTag (Variables|Default|GetAbilitySystemComponent) (GameplayTags|MakeLiteralGameplayTagContainer "(GameplayTags=((TagName=\"Ability.HitReaction.Front\")))") true)
        (else
          (Abilities|TryActivateAbilitiesbyTag (Variables|Default|GetAbilitySystemComponent) (GameplayTags|MakeLiteralGameplayTagContainer "(GameplayTags=((TagName=\"Ability.HitReaction.Back\")))") true))))))

(event Input|KeyboardEvents|DebugKeyT
  (params (Key :type Key%20Structure :default "None") (ActionValue :type Input%20Action%20Value%20Structure))
  (:Pressed
    (GameplayEffects|ApplyGameplayEffectToSelf :self (Variables|Default|GetAbilitySystemComponent) :GameplayEffectClass "/Game/Blueprint/GameplayEffect/GE_Damage.GE_Damage_C")))

(event Input|KeyboardEvents|K
  (params (Key :type Key%20Structure :default "None"))
  (:Pressed
    (CallFunction|PerformDead)))

(fn ConstructionScript)

(fn Vault
  (bind _index (Utilities|FlowControl|ForLoopwithBreak 0 2 :!label _label)
    (:LoopBody
      (bind (_outhit _returnvalue) (Collision|SphereTraceByChannel (+ (Transformation|GetActorLocation) (Math|Vector|MakeVector 0.0 0.0 (* _index 30))) (+ (+ (Transformation|GetActorLocation) (Math|Vector|MakeVector 0.0 0.0 (* _index 30))) (* (Math|Vector|GetForwardVector (Transformation|GetActorRotation)) 1.8e+02)) 5.0 "TraceTypeQuery1" false 0 "ForDuration"))
      (if _returnvalue
        ;[1 1 1] 여기서 해당 연산을 끝내고 왜 트레이스의 경로가 바뀌는지 잘 모르겠음.
        (Utilities|FlowControl|Sequence
          (:then_0
            (goto _label Break))
          (:then_1
            (bind _index_2 (Utilities|FlowControl|ForLoopwithBreak 0 5 :!label _label_2)
              (:LoopBody
                (bind (_outhit_2 _returnvalue_2) (Collision|SphereTraceByChannel (+ (+ (.Location (Collision|BreakHitResult _outhit)) "0.000000,0.000000,100.000000") (* (* _index_2 50) (Math|Vector|GetForwardVector (Transformation|GetActorRotation)))) (- (+ (+ (.Location (Collision|BreakHitResult _outhit)) "0.000000,0.000000,100.000000") (* (* _index_2 50) (Math|Vector|GetForwardVector (Transformation|GetActorRotation)))) "0.000000,0.000000,100.000000") 1e+01 "TraceTypeQuery1" false 0 "ForDuration"))
                (if _returnvalue_2
                  ;[1 1 1] 트레이스의 첫번째 지점을 확인하여 모션워핑에 사용합니다.
                  (Utilities|FlowControl|Sequence
                    (:then_0
                      (if (== _index_2 0)
                        (bind _output_get (Variables|Vault|SetVault%20Start%20Pos (.Location (Collision|BreakHitResult _outhit_2))))
                        (Rendering|Debug|DrawDebugSphere _output_get 1e+01 12 "(R=1.000000,G=0.076905,B=0.832584,A=1.000000)" 1e+01 2.0)))
                    (:then_1
                      (bind _output_get_2 (Variables|Vault|SetVault%20Middle%20Pos (.Location (Collision|BreakHitResult _outhit_2))))
                      (Rendering|Debug|DrawDebugSphere _output_get_2 1e+01 12 "(R=1.000000,G=0.993149,B=0.000000,A=1.000000)" 1e+01 2.0)
                      (Variables|Vault|SetCan%20Warp true)))
                  (else
                    (bind (_outhit_3 _returnvalue_3) (Collision|LineTraceByChannel (+ (.TraceStart (Collision|BreakHitResult _outhit_2)) (* (Math|Vector|GetForwardVector (Transformation|GetActorRotation)) 8e+01)) (- (+ (.TraceStart (Collision|BreakHitResult _outhit_2)) (* (Math|Vector|GetForwardVector (Transformation|GetActorRotation)) 8e+01)) "0.000000,0.000000,1000.000000") "TraceTypeQuery1" false 0 "ForDuration" true "(R=0.009740,G=0.000000,B=1.000000,A=1.000000)"))
                    (if _returnvalue_3
                      (Variables|Vault|SetVault%20Land%20Pos (.Location (Collision|BreakHitResult _outhit_3)))
                      (goto _label_2 Break)))))
              (:Completed
                (CallFunction|VaultMotionWarp)))))))))

(fn Blocking
  (Class|CharaterAnimInstance|SetIsBlocking (Variables|Default|GetAnimInstance) true))

(fn FinishedBlocking
  (Class|CharaterAnimInstance|SetIsBlocking (Variables|Default|GetAnimInstance) false))

(fn TargetLook)

(fn SetPlayerRotate
  (bind _charactermovement (Variables|Character|GetCharacterMovement))
  (bind _returnvalue (Pawn|Components|CharacterMovement|GetCurrentAcceleration _charactermovement))
  (if (> (Math|Vector|VectorLength _returnvalue) 0.0)
    (Transformation|SetActorRotation (Math|Interpolation|RInterpTo (Transformation|GetActorRotation) (Math|Rotator|MakeRotator 0.0 0.0 (+ (.Yaw (Math|Rotator|BreakRotator (Pawn|GetControlRotation :!class /Script/Engine.Pawn))) (Math|Curves|GetFloatValue (Variables|Default|GetDirectionCurve) (.Yaw (Math|Rotator|BreakRotator (Math|Rotator|Delta(Rotator) (Math|Rotator|MakeRotfromX _returnvalue) (Pawn|GetControlRotation :!class /Script/Engine.Pawn))))))) (Utilities|Time|GetWorldDeltaSeconds) 1e+01))))

(fn CanReciveDamage
  (return (not (Variables|Default|GetIFrame))))