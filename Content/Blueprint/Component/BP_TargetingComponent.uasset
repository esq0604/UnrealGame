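; Actor component that gives a player-controlled character a toggleable lock-on camera aimed at a target actor.
; Enabling runs a sphere trace along the follow camera's forward direction, accepting a hit actor that implements BPI_Targeting.
; While locked, Tick interpolates controller pitch and yaw toward just below the target's location, releasing when it becomes invalid or untargetable.
; UpdateRotationMode is an empty stub, and debug prints and trace drawing remain active.
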(event EventBeginPlay
  (bind _as캐릭터 (Utilities|Casting|CastToCharacter (Components|GetOwner)))
  (Variables|Default|SetOwnerCharacter _as캐릭터)
  (bind _as플레이어_컨트롤러 (Utilities|Casting|CastToPlayerController (Pawn|GetController (Variables|Default|GetOwnerCharacter))))
  (Variables|Default|SetOwnerController _as플레이어_컨트롤러)
  (Variables|Default|SetFollowCamera (Actor|GetComponentbyClass (Variables|Default|GetOwnerCharacter) "/Script/Engine.CameraComponent")))

(event EventTick
  (params (DeltaSeconds :type Float%20%28single-precision%29))
  (if (Variables|Default|GetIsTargeting)
    (CallFunction|UpdateTargetingControlRotation)))

(fn FindTarget
  (bind _returnvalue (Components|GetOwner))
  (bind _targetting_distance (Variables|Default|GetTargetting%20Distance))
  (bind _followcamera (Variables|Default|GetFollowCamera))
  (bind _returnvalue_2 (Transformation|GetActorLocation _returnvalue))
  (bind _returnvalue_3 (Math|Vector|GetForwardVector _followcamera))
  (bind _returnvalue_4 (* _returnvalue_3 _targetting_distance))
  (bind (_outhit _returnvalue_5) (Collision|SphereTraceForObjects _returnvalue_2 (+ _returnvalue_2 (Math|Vector|MakeVector (.x _returnvalue_4) (.y _returnvalue_4) (Variables|Default|GetzOffset))) (Variables|Default|GetTargetting%20Radius) (Variables|Default|GetTarget%20Object%20Types) false (Utilities|Array|MakeArray (Components|GetOwner)) "ForDuration"))
  (if (and _returnvalue_5 (Utilities|IsValid (.HitActor (Collision|BreakHitResult _outhit))))
    (if (Utilities|DoesObjectImplementInterface (.HitActor (Collision|BreakHitResult _outhit)) "/Game/Blueprint/Interface/BPI_Targeting.BPI_Targeting_C")
      (return true (.HitActor (Collision|BreakHitResult _outhit)))
      (else
        _)))
  (return false 0))

(fn UpdateTargetingControlRotation
  (bind _returnvalue (Utilities|Time|GetWorldDeltaSeconds))
  (bind _returnvalue_2 (Components|GetOwner))
  (bind _targetactor (Variables|Default|GetTargetActor))
  (bind _ownercontroller (Variables|Default|GetOwnerController))
  (bind _target_rotation_interp_speed (Variables|Default|GetTarget%20Rotation%20Interp%20Speed))
  (bind _returnvalue_3 (Transformation|GetActorLocation _targetactor))
  (bind _returnvalue_4 (Transformation|GetActorLocation _returnvalue_2))
  (bind _returnvalue_5 (Transformation|GetActorRotation _ownercontroller))
  (bind _returnvalue_6 (- _returnvalue_3 "0.000000,0.000000,50.000000"))
  (bind _returnvalue_7 (Math|Rotator|FindLookatRotation _returnvalue_4 _returnvalue_6))
  (bind _returnvalue_8 (Math|Interpolation|RInterpTo _returnvalue_5 _returnvalue_7 _returnvalue _target_rotation_interp_speed))
  (if (and (Utilities|IsValid (Variables|Default|GetOwnerController)) (Utilities|IsValid (Variables|Default|GetTargetActor)))
    (bind _returnvalue_9 (Class|BPITargeting|CanbeTargeted?(Message) (Variables|Default|GetTargetActor)))
    (if _returnvalue_9
      (Pawn|SetControlRotation (Variables|Default|GetOwnerController) (Math|Rotator|MakeRotator (.Roll (Math|Rotator|BreakRotator _returnvalue_5)) (.pitch _returnvalue_8) (.yaw _returnvalue_8)))
      (else
        (CallFunction|DisableLockon :!label _label)))
    (else
      (goto _label))))

(fn DisableLockon
  (CallFunction|SetIsTargeting false)
  (CallFunction|SetTargetActor)
  (CallFunction|UpdateRotationMode))

(fn EnableLockon
  (bind (_returnvalue _foundtarget) (CallFunction|FindTarget))
  (if _returnvalue
    (CallFunction|SetTargetActor _foundtarget)
    (CallFunction|SetIsTargeting true)))

(fn SetTargetActor
  (params (NewParam :type Actor%20Object%20Reference))
  (Variables|Default|SetTargetActor NewParam))

(fn SetIsTargeting
  (params (EnableTargeting :type Boolean))
  (Variables|Default|SetIsTargeting EnableTargeting)
  (bind _targetactor (Variables|Default|GetTargetActor)
    (:then
      (Development|PrintString (Utilities|GetDisplayName _targetactor)))
    (:else)))

(fn ToggleLockon
  (Development|PrintString (Utilities|String|ToString(Boolean) (Variables|Default|GetIsTargeting)))
  (if (Variables|Default|GetIsTargeting)
    (CallFunction|DisableLockon)
    (else
      (CallFunction|EnableLockon))))

(fn UpdateRotationMode)