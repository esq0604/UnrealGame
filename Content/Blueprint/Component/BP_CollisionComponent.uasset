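; BP_CollisionComponent is a component that detects weapon hits while its collision flag is enabled.
; Each Tick, it runs a multi-sphere object trace between the WeaponStart and WeaponEnd sockets of an externally assigned mesh component.
; Each actor is recorded on first hit and broadcast through OnHit, so it registers only once per activation.
; Enabling collision through SetCollisionEnable clears that list for a new swing.
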(event Custom|CollisionEnable
  (bind _collisionmeshcomponent (Variables|Default|GetCollisionMeshComponent))
  ;[0 0 0 1 20] CollisionEnable
  (bind _outhits (Collision|MultiSphereTraceForObjects (Transformation|GetSocketLocation _collisionmeshcomponent (Variables|Initialization|GetWeaponStart)) (Transformation|GetSocketLocation _collisionmeshcomponent (Variables|Initialization|GetWeaponEnd)) (Variables|Initialization|GetTraceRadius) (Variables|Initialization|GetTraceObjectTypes) false (Variables|Initialization|GetActorsToIgnore) (Variables|Initialization|GetDrawDebugType)))
  (for _array_element _outhits
    (bind _output_get (Variables|Default|SetLastHit _array_element))
    (if (CallFunction|CanHitActor (.HitActor (Collision|BreakHitResult _output_get)))
      (bind _output_get_2 (Variables|Default|SetHit%20Actor (.HitActor (Collision|BreakHitResult _output_get))))
      (Utilities|Array|AddUnique (Variables|Default|GetAlreadyHitActor) _output_get_2)
      (Default|CallOnHit _output_get))))

(event Custom|SetCollisionMeshComp
  (params (CollisionMeshComponent :type Primitive%20Component%20Object%20Reference))
  ;[0 0 0 1 20] Setter
  (Variables|Default|SetCollisionMeshComponent CollisionMeshComponent))

(event Custom|SetCollisionEnable
  (params (bCollisionEnable :type Boolean))
  ;[0 0 0 1 20] Setter
  (if bCollisionEnable
    (Utilities|Array|Clear (Variables|Default|GetAlreadyHitActor))
    (Variables|Default|SetbCollisionEnable true)
    (else
      (Variables|Default|SetbCollisionEnable false))))

(event EventBeginPlay)

(event EventTick
  (params (DeltaSeconds :type Float%20%28single-precision%29))
  (if (Variables|Default|GetbCollisionEnable)
    (CallFunction|CollisionEnable)))

(fn CanHitActor
  (params (CheckActor :type Actor%20Object%20Reference))
  (return (not (Utilities|Array|ContainsItem (Variables|Default|GetAlreadyHitActor) CheckActor))))