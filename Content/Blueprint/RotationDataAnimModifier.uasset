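; Animation modifier that bakes root bone yaw into a float curve on an animation sequence.
; On apply, it adds a curve named RotationCurve, then loops over the frames of the sequence.
; Each frame gets a key at its time, valued with the root bone's yaw sampled with root motion extraction enabled.
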(event EventOnApply
  (params (AnimationSequence :type Anim%20Sequence%20Object%20Reference))
  (bind _output_get (Variables|Default|SetAnimation%20Sequence AnimationSequence))
  (Class|AnimationBlueprintLibrary|AddCurve _output_get "RotationCurve" "RCT_Float" false)
  (for _index (range 0 (Class|AnimationBlueprintLibrary|GetNumFrames (Variables|Default|GetAnimation%20Sequence)))
    (Variables|Default|SetLoopIndex _index)
    (Class|AnimationBlueprintLibrary|AddFloatCurveKey (Variables|Default|GetAnimation%20Sequence) "RotationCurve" (Class|AnimationBlueprintLibrary|GetTimeatFrame (Variables|Default|GetAnimation%20Sequence) (Variables|Default|GetLoopIndex)) (.Yaw (Math|Rotator|BreakRotator (.rotation (Class|AnimationBlueprintLibrary|GetBonePoseforFrame (Variables|Default|GetAnimation%20Sequence) "root" (Variables|Default|GetLoopIndex) true)))))))