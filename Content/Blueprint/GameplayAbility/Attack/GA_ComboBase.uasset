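; Base Gameplay Ability for a player combo attack that plays a configurable montage.
; On activation it commits, caches the BP_Player owner and requires a BP_CustomPlayerController.
; A first attack plays its montage immediately, while a follow-up first waits for a single Ability.State.NextAttack gameplay event.
; The ability ends when the montage completes, blends out, is interrupted or is cancelled.
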(event Ability|EventActivateAbility
  (bind _returnvalue (Ability|GetActorInfo))
  (bind (_owneractor _avataractor _playercontroller) (Utilities|Struct|BreakGameplayAbilityActorInfo _returnvalue))
  (Ability|CommitAbility)
  (bind _asbp_player (Utilities|Casting|CastToBP_Player _owneractor))
  (Variables|Default|SetAs%20BP%20Player _asbp_player)
  (Utilities|Casting|CastToBP_CustomPlayerController _playercontroller)
  (if (Variables|Default|GetIsFirstAttack)
    _
    (else
      (Ability|Tasks|WaitGameplayEvent "(TagName=\"Ability.State.NextAttack\")" 0 true
        (:EventReceived
          _))))
  (|PlayMontageandWaitProxy "None" (Variables|Default|GetMontage%20to%20Play) 1.0 "None" true 1.0 0.0
    (:OnCompleted
      _)
    (:OnBlendOut
      _)
    (:OnInterrupted
      _)
    (:OnCancelled
      _))
  (Ability|EndAbility))