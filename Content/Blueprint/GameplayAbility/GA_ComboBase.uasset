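; Base gameplay ability for one attack step in the player's combo, playing a configurable montage.
; A first attack starts immediately, while any other step waits for a single Ability.State.NextAttack gameplay event.
; Before playing the montage, it sets the player's AttackTarget motion warp point a short distance straight ahead.
; The ability ends when the montage completes, blends out, is interrupted or is cancelled.
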(event Ability|EventActivateAbility
  (bind _asbp_player (Utilities|Casting|CastToBP_Player (.OwnerActor (Utilities|Struct|BreakGameplayAbilityActorInfo (Ability|GetActorInfo)))))
  (if (Variables|Default|GetIsFirstAttack)
    _
    (else
      (Ability|Tasks|WaitGameplayEvent "(TagName=\"Ability.State.NextAttack\")" 0 true
        (:EventReceived
          _))))
  (Class|MotionWarpingComponent|AddorUpdateWarpTarget (Variables|/Script/RetargetingTest.CharacterBase|GetMotionWarpComponent _asbp_player) (Utilities|Struct|MakeMotionWarpingTarget "AttackTarget" (+ (* (Transformation|GetActorForwardVector _asbp_player) 1e+02) (Transformation|GetActorLocation _asbp_player)) "0.000000,0.000000,0.000000" 0 "None" false))
  (|PlayMontageandWaitProxy "None" (Variables|Default|GetMontage%20to%20Play) 1.0 "None" true 1.0 0.0
    (:OnCompleted
      _)
    (:OnBlendOut
      _)
    (:OnInterrupted
      _)
    (:OnCancelled
      _))
  (Ability|EndAbility))

(event Ability|EventOnEndAbility
  (params (bWasCancelled :type Boolean)))