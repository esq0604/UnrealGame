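; Gameplay ability that toggles the player's weapon equip state with a montage.
; On activation it commits, casts the owner actor to BP_Player, then branches on IsAttachedWeapon to play a montage on the player's mesh.
; Each branch flips the flag as soon as playback is launched, and completion, blend-out or interruption ends the ability.
; The graph itself performs no attachment, and a failed cast stops without ending the ability.
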(event Ability|EventActivateAbility
  (Ability|CommitAbility)
  (bind _asbp_player (Utilities|Casting|CastToBP_Player (.OwnerActor (Utilities|Struct|BreakGameplayAbilityActorInfo (Ability|GetActorInfo)))))
  (if (Variables|Default|GetIsAttachedWeapon)
    (Animation|Montage|PlayMontage (Variables|/Script/Engine.Character|GetMesh _asbp_player) 0
      (:then
        (Variables|Default|SetIsAttachedWeapon false))
      (:OnCompleted
        (Ability|EndAbility :!label _label))
      (:OnBlendOut
        (goto _label))
      (:OnInterrupted
        (goto _label)))
    (else
      (Animation|Montage|PlayMontage (Variables|/Script/Engine.Character|GetMesh _asbp_player) 0
        (:then
          (Variables|Default|SetIsAttachedWeapon true))
        (:OnCompleted
          (goto _label))
        (:OnBlendOut
          (goto _label))
        (:OnInterrupted
          (goto _label))))))

(event Ability|EventOnEndAbility
  (params (bWasCancelled :type Boolean)))