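; GA_Block is a gameplay ability that puts the player character into a blocking state.
; On activation it commits, applies the GE_StateBlock effect to its owner, and calls Blocking on BP_Player.
; A WaitGameplayTagRemove task ends the ability once the Character.IsBlocking tag is removed.
; When the ability ends, it calls FinishedBlocking on the player and ends the stored wait task.
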(event Ability|EventActivateAbility
  (Ability|CommitAbility)
  (Ability|ApplyGameplayEffectToOwner "/Game/Blueprint/GameplayEffect/GE_StateBlock.GE_StateBlock_C")
  ;[1 1 1] 코멘트
  (bind _asbp_player (Utilities|Casting|CastToBP_Player (.OwnerActor (Utilities|Struct|BreakGameplayAbilityActorInfo (Ability|GetActorInfo)))))
  (Default|Blocking _asbp_player)
  (bind _asynctaskproxy (Ability|Tasks|WaitGameplayTagRemove "(TagName=\"Character.IsBlocking\")" 0 true)
    (:then
      (Variables|Default|SetWait%20For%20Tag%20Remove _asynctaskproxy))
    (:Removed
      (Ability|EndAbility))))

(event Ability|EventOnEndAbility
  (params (bWasCancelled :type Boolean))
  (bind _wait_for_tag_remove (Variables|Default|GetWait%20For%20Tag%20Remove))
  ;[1 1 1] 코멘트
  (Default|FinishedBlocking (stale Ability|EventActivateAbility _asbp_player))
  (Utilities|IsValid _wait_for_tag_remove
    (:Is%20Valid
      (GameplayTasks|EndTask _wait_for_tag_remove))))