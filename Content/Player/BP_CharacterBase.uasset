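; Base character Blueprint that exposes health, mana and stamina from its Ability System Component.
; Each getter reads a float attribute from the component, and a paired ratio function divides that result by the matching Max variable, with no zero check.
; Blocking and Finished Blocking are empty functions, and the event graph and construction script hold no logic.
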(event EventBeginPlay)

(event Collision|EventActorBeginOverlap
  (params (OtherActor :type Actor%20Object%20Reference)))

(event EventTick
  (params (DeltaSeconds :type Float%20%28single-precision%29)))

(fn ConstructionScript)

(fn Blocking)

(fn FinishedBlocking)

(fn GetHealth
  (return (.ReturnValue (Ability|Attribute|GetFloatAttributefromAbilitySystemComponent (Variables|Default|GetAbilitySystemComponent) "(AttributeName=\"Health\",Attribute=/Script/RetargetingTest.RuneAttributeSet:Health,AttributeOwner=/Script/CoreUObject.Class'\"/Script/RetargetingTest.RuneAttributeSet\"')"))))

(fn GetHealthasRatio
  (bind _result (CallFunction|GetHealth))
  (return (/ _result (Variables|Default|GetMaxHealth))))

(fn GetMana
  (return (.ReturnValue (Ability|Attribute|GetFloatAttributefromAbilitySystemComponent (Variables|Default|GetAbilitySystemComponent) "(AttributeName=\"Mana\",Attribute=/Script/RetargetingTest.RuneAttributeSet:Mana,AttributeOwner=/Script/CoreUObject.Class'\"/Script/RetargetingTest.RuneAttributeSet\"')"))))

(fn GetManaasRatio
  (bind _result (CallFunction|GetMana))
  (return (/ _result (Variables|Default|GetMaxMana))))

(fn GetStamina
  (return (.ReturnValue (Ability|Attribute|GetFloatAttributefromAbilitySystemComponent (Variables|Default|GetAbilitySystemComponent) "(AttributeName=\"Stamina\",Attribute=/Script/RetargetingTest.RuneAttributeSet:Stamina,AttributeOwner=/Script/CoreUObject.Class'\"/Script/RetargetingTest.RuneAttributeSet\"')"))))

(fn GetStaminaasRatio
  (bind _result (CallFunction|GetStamina))
  (return (/ _result (Variables|Default|GetMaxStamina))))