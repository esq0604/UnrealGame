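; Gameplay ability that toggles the player's twinblades between equipped and unarmed by playing the matching montage on the BP_Player mesh.
; The ability's IsAttachedWeapon flag picks the equip or unarm montage and flips as playback starts; no weapon attachment happens in this graph.
; It uses plain PlayMontage rather than a montage ability task, ending on completion, blend out or interruption.
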(event Ability|EventActivateAbility
  (Ability|CommitAbility)
  (bind _asbp_player (Utilities|Casting|CastToBP_Player (.OwnerActor (Utilities|Struct|BreakGameplayAbilityActorInfo (Ability|GetActorInfo)))))
  (if (Variables|Default|GetIsAttachedWeapon)
    (Animation|Montage|PlayMontage (Variables|/Script/Engine.Character|GetMesh _asbp_player) "/Game/Asset/Animation/TwinbladesExpansion/TwinbladesExpansion/Common/Inplace/Twinblades_Equip_Montage.Twinblades_Equip_Montage"
      (:then
        (Variables|Default|SetIsAttachedWeapon false))
      (:OnCompleted
        (Ability|EndAbility :!label _label))
      (:OnBlendOut
        (goto _label))
      (:OnInterrupted
        (goto _label)))
    (else
      (Animation|Montage|PlayMontage (Variables|/Script/Engine.Character|GetMesh _asbp_player) "/Game/Asset/Animation/TwinbladesExpansion/TwinbladesExpansion/Common/Inplace/Twinblades_Unarm_Montage1.Twinblades_Unarm_Montage1"
        (:then
          (Variables|Default|SetIsAttachedWeapon true))
        (:OnCompleted
          (goto _label))
        (:OnBlendOut
          (goto _label))
        (:OnInterrupted
          (goto _label))))))

(event Ability|EventOnEndAbility
  (params (bWasCancelled :type Boolean)))