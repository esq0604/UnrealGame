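; GA_Block is a gameplay ability that puts a player character into a blocking state.
; On activation it commits, applies GE_IsBlocking to the owner, calls Blocking on the BP_CharacterBase owner, then waits for the Character.IsBlocking tag to be removed.
; Tag removal ends the ability, which calls FinishedBlocking on the character and ends the stored wait task.
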(event Ability|EventActivateAbility
  (Ability|CommitAbility)
  (Ability|ApplyGameplayEffectToOwner "/Game/Player/GameplayEffect/GE_IsBlocking.GE_IsBlocking_C")
  (bind _asbp_character_base (Utilities|Casting|CastToBP_CharacterBase (.OwnerActor (Utilities|Struct|BreakGameplayAbilityActorInfo (Ability|GetActorInfo)))))
  (Default|Blocking _asbp_character_base)
  (bind _asynctaskproxy (Ability|Tasks|WaitGameplayTagRemove "(TagName=\"Character.IsBlocking\")" 0)
    (:then
      (Variables|Default|SetWait%20For%20Tag%20Remove _asynctaskproxy))
    (:Removed
      (Ability|EndAbility))))

(event Ability|EventOnEndAbility
  (params (bWasCancelled :type Boolean))
  (bind _wait_for_tag_remove (Variables|Default|GetWait%20For%20Tag%20Remove))
  (Default|FinishedBlocking (stale Ability|EventActivateAbility _asbp_character_base))
  (Utilities|IsValid _wait_for_tag_remove
    (:Is%20Valid
      (GameplayTasks|EndTask _wait_for_tag_remove))))